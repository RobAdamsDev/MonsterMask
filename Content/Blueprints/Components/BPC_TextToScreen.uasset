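; Actor component that shows tutorial text on screen through a TextToScreen function.
; It removes the tutorial widget tracked by GM_YDBH, then creates a new one with the given read duration and registers it there.
; The game mode's current input type selects keyboard/mouse or gamepad text.
; The color parameter is currently unused, so text and bar take a default color before the widget joins the viewport.
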(event EventBeginPlay)

(fn TexttoScreen
  (params (TutorialText :type Text) (TutorialText_GamePad :type Text) (Tutorial%20Color%20and%20Opacity :type Slate%20Color%20Structure) (ReadDuration :type Float%20%28single-precision%29))
  (bind _default_color (Variables|Default|Getdefault%20color))
  (bind _asgm_ydbh (Utilities|Casting|CastToGM_YDBH (Game|GetGameMode)))
  (Variables|Default|SetGameMode _asgm_ydbh)
  (if (Utilities|IsValid (Variables|/Game/Blueprints/Game/GM_YDBH.GM_YDBH_C|GetTutorialOnScreen (Variables|Default|GetGameMode)))
    (Widget|RemovefromParent (Variables|/Game/Blueprints/Game/GM_YDBH.GM_YDBH_C|GetTutorialOnScreen (Variables|Default|GetGameMode))))
  (bind _returnvalue (UserInterface|CreateWidget "/Game/UI/Widgets/TutorialWidget.TutorialWidget_C" (Game|GetPlayerController 0) "FullText" "" ReadDuration))
  (bind _output_get (Variables|Default|SetWidgetRef _returnvalue))
  (Variables|/Game/Blueprints/Game/GM_YDBH.GM_YDBH_C|SetTutorialOnScreen (Variables|Default|GetGameMode) _output_get)
  (switch Utilities|FlowControl|Switch|SwitchonECommonInputType (Variables|/Game/Blueprints/Game/GM_YDBH.GM_YDBH_C|GetCurrentInputType (Variables|Default|GetGameMode))
    (:MouseAndKeyboard
      (Variables|/Game/UI/Widgets/TutorialWidget.TutorialWidget_C|SetFullText (Variables|Default|GetWidgetRef) TutorialText))
    (:Gamepad
      (Variables|/Game/UI/Widgets/TutorialWidget.TutorialWidget_C|SetFullText (Variables|Default|GetWidgetRef) TutorialText_GamePad)))
  (Appearance|SetColorandOpacity (Variables|/Game/UI/Widgets/TutorialWidget.TutorialWidget_C|GetTutorialText (Variables|Default|GetWidgetRef)) _default_color :!class /Script/UMG.TextBlock)
  (Appearance|SetColorandOpacity (Variables|/Game/UI/Widgets/TutorialWidget.TutorialWidget_C|GetBar (Variables|Default|GetWidgetRef)) (.SpecifiedColor (Utilities|Struct|BreakSlateColor _default_color)) :!class /Script/UMG.Image)
  (Class|Widget|SetRenderTransformPivot (Variables|/Game/UI/Widgets/TutorialWidget.TutorialWidget_C|GetBar (Variables|Default|GetWidgetRef)))
  (Class|Widget|SetRenderTransform (Variables|/Game/UI/Widgets/TutorialWidget.TutorialWidget_C|GetBar (Variables|Default|GetWidgetRef)) (Utilities|Struct|MakeWidgetTransform "(X=0.000000,Y=0.000000)" (Math|Vector2D|MakeVector2D 1.0 (Variables|Default|GetBarScale)) "(X=0.000000,Y=0.000000)" 0.0))
  (UserInterface|Viewport|AddtoViewport (Variables|Default|GetWidgetRef) 0))