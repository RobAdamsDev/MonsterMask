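; BP_Tutorial is a trigger volume that shows tutorial text on screen when the player overlaps it.
; Its construction script sizes the box from the BoxExtent variable.
; Unless Hidden is set, a DoOnce gates the overlap, then after a short delay BPCTextToScreen displays the keyboard or gamepad text with its color and read duration.
; After a cooldown it either destroys itself or resets the gate to show again.
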(event OnComponentBeginOverlap(Box)
  (params (OverlappedComponent :type Primitive%20Component%20Object%20Reference) (OtherActor :type Actor%20Object%20Reference) (OtherComp :type Primitive%20Component%20Object%20Reference) (OtherBodyIndex :type Integer) (bFromSweep :type Boolean) (SweepResult :type Hit%20Result%20Structure%20%28by%20ref%29))
  (Utilities|Casting|CastToBP_Player OtherActor)
  (if (not (Variables|Rendering|GetbHidden))
    (Utilities|FlowControl|DoOnce false :!label _label
      (:Completed
        (Utilities|FlowControl|Delay 0.33)
        (Default|TexttoScreen (Variables|Default|GetBPC_TextToScreen) (Variables|1.Tutorial|GetTutorialText) (Variables|1.Tutorial|GetTutorialText_GamePad) (Variables|1.Tutorial|GetTutorial%20Color%20and%20Opacity) (Variables|1.Tutorial|GetRead%20Duration))
        (Utilities|FlowControl|Delay 1e+01)
        (if (Variables|1.Tutorial|GetOnlyShowOnce?)
          (Actor|DestroyActor)
          (else
            (goto _label Reset)))))))

(fn ConstructionScript
  (Components|Box|SetBoxExtent (Variables|Default|GetBox) (Variables|1.Tutorial|GetBox%20Extent) true))